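; BP_CustomizeActor is a modular character for clothing customization, built from separate body and clothing skeletal meshes that follow one master pose component set in the Construction Script.
; On BeginPlay it dresses itself from the "charsave" CharacterSave slot, or from a newly created save object if none exists.
; UpdateClothing swaps the pants, balaclava, jacket or body mesh by flag, clearing the jacket when JacketVisible is false; it neither changes shoes nor saves.
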(event Custom|UpdateClothing
  (params (Leg? :type Boolean) (Face? :type Boolean) (Mesh :type Skeletal%20Mesh%20Object%20Reference) (Jacket? :type Boolean) (Body? :type Boolean) (JacketVisible? :type Boolean))
  (if Leg?
    (Class|SkinnedMeshComponent|SetSkeletalMesh (Variables|Default|GetSK_Man_Pants) Mesh true)
    (if (not JacketVisible?) :!label _label
      (Class|SkinnedMeshComponent|SetSkeletalMesh (Variables|Default|GetSK_Man_Jacket) 0 true))
    (elif Face?
      (Class|SkinnedMeshComponent|SetSkeletalMesh (Variables|Default|GetSK_Man_Balaclava) Mesh true)
      (goto _label)
      (elif Jacket?
        (Class|SkinnedMeshComponent|SetSkeletalMesh (Variables|Default|GetSK_Man_Jacket) Mesh true)
        (goto _label)
        (elif Body?
          (Class|SkinnedMeshComponent|SetSkeletalMesh (Variables|Default|GetSK_Man_Body_For_Jacket) Mesh true)
          (goto _label))))))

(event EventBeginPlay
  (bind _returnvalue (SaveGame|DoesSaveGameExist "charsave"))
  (if _returnvalue
    (bind _returnvalue_2 (SaveGame|LoadGamefromSlot "charsave"))
    (bind _output_get (Variables|Default|SetSaveGame _returnvalue_2))
    (bind _ascharacter_save (Utilities|Casting|CastToCharacterSave _output_get))
    (Class|SkinnedMeshComponent|SetSkeletalMesh (Variables|Default|GetSK_Man_Shoes) (Variables|/Game/CharacterSave.CharacterSave_C|GetShoes _ascharacter_save) true)
    (Class|SkinnedMeshComponent|SetSkeletalMesh (Variables|Default|GetSK_Man_Pants) (Variables|/Game/CharacterSave.CharacterSave_C|GetLegs _ascharacter_save) true)
    (Class|SkinnedMeshComponent|SetSkeletalMesh (Variables|Default|GetSK_Man_Balaclava) (Variables|/Game/CharacterSave.CharacterSave_C|GetFaceAcessory _ascharacter_save) true)
    (Class|SkinnedMeshComponent|SetSkeletalMesh (Variables|Default|GetSK_Man_Body_For_Jacket) (Variables|/Game/CharacterSave.CharacterSave_C|GetBodyMesh _ascharacter_save) true)
    (Class|SkinnedMeshComponent|SetSkeletalMesh (Variables|Default|GetSK_Man_Jacket) (Variables|/Game/CharacterSave.CharacterSave_C|GetJacket _ascharacter_save) true)
    (else
      (bind _returnvalue_3 (SaveGame|CreateSaveGameObject "/Game/CharacterSave.CharacterSave_C"))
      (Variables|Default|SetSaveGame _returnvalue_3)
      (Class|SkinnedMeshComponent|SetSkeletalMesh (Variables|Default|GetSK_Man_Shoes) (Variables|/Game/CharacterSave.CharacterSave_C|GetShoes _returnvalue_3) true)
      (Class|SkinnedMeshComponent|SetSkeletalMesh (Variables|Default|GetSK_Man_Pants) (Variables|/Game/CharacterSave.CharacterSave_C|GetLegs _returnvalue_3) true)
      (Class|SkinnedMeshComponent|SetSkeletalMesh (Variables|Default|GetSK_Man_Balaclava) (Variables|/Game/CharacterSave.CharacterSave_C|GetFaceAcessory _returnvalue_3) true)
      (Class|SkinnedMeshComponent|SetSkeletalMesh (Variables|Default|GetSK_Man_Body_For_Jacket) (Variables|/Game/CharacterSave.CharacterSave_C|GetBodyMesh _returnvalue_3) true)
      (Class|SkinnedMeshComponent|SetSkeletalMesh (Variables|Default|GetSK_Man_Jacket) (Variables|/Game/CharacterSave.CharacterSave_C|GetJacket _returnvalue_3) true))))

(fn ConstructionScript
  (Class|SkinnedMeshComponent|SetMasterPoseComponent (Variables|Default|GetSK_Man_Balaclava) (Variables|Default|GetSkeletalMesh) false))